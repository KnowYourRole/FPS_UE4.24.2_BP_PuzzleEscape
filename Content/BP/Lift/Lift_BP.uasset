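; Lift Blueprint whose platform rises when a Cube2 object is on its trigger and the first-person character is inside the player check collider.
; Overlap events on both volumes set two flags, and both being true plays a timeline that lerps the lift mesh between start and end points.
; An end overlap reverses the timeline only if the other flag is still true.
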(event OnComponentEndOverlap(Trigger)
  (params (OverlappedComponent :type Primitive%20Component%20Object%20Reference) (OtherActor :type Actor%20Object%20Reference) (OtherComp :type Primitive%20Component%20Object%20Reference) (OtherBodyIndex :type Integer))
  ;[1 1 1] When the player removes the object from the trigger it activates the revers and the platform goes down
  (Utilities|Casting|CastToCube2 OtherActor)
  (bind _output_get (Variables|Default|SetCubeIsTrue false))
  (if (or _output_get (stale OnComponentEndOverlap(PlayerCheckCollider) _output_get))
    (bind _newtrack_0 (Timeline|Timeline_0 Reverse)
      (:Update
        (Transformation|SetRelativeLocation (Variables|Default|GetLiftMesh) (Math|Vector|Lerp(Vector) (Variables|Default|GetStart%20Point) (Variables|Default|GetEnd%20Point) _newtrack_0) false false)))))

(event OnComponentEndOverlap(PlayerCheckCollider)
  (params (OverlappedComponent :type Primitive%20Component%20Object%20Reference) (OtherActor :type Actor%20Object%20Reference) (OtherComp :type Primitive%20Component%20Object%20Reference) (OtherBodyIndex :type Integer))
  (Utilities|Casting|CastToFirstPersonCharacter OtherActor)
  (bind _output_get (Variables|Default|SetPlayerIsTrue false))
  (if (or (stale OnComponentEndOverlap(Trigger) _output_get) _output_get)
    (bind _newtrack_0 (Timeline|Timeline_0 Reverse)
      (:Update
        (Transformation|SetRelativeLocation (Variables|Default|GetLiftMesh) (Math|Vector|Lerp(Vector) (Variables|Default|GetStart%20Point) (Variables|Default|GetEnd%20Point) _newtrack_0) false false)))))

(event OnComponentBeginOverlap(Trigger)
  (params (OverlappedComponent :type Primitive%20Component%20Object%20Reference) (OtherActor :type Actor%20Object%20Reference) (OtherComp :type Primitive%20Component%20Object%20Reference) (OtherBodyIndex :type Integer) (bFromSweep :type Boolean) (SweepResult :type Hit%20Result%20Structure%20%28by%20ref%29))
  ;[1 1 1] When the object is placed on the trigger, the platform goes up
  (Utilities|Casting|CastToCube2 OtherActor)
  (Variables|Default|SetCubeIsTrue true)
  (if (and (Variables|Default|GetCubeIsTrue) (Variables|Default|GetPlayerIsTrue))
    (bind _newtrack_0 (Timeline|Timeline_0 Play)
      (:Update
        (Transformation|SetRelativeLocation (Variables|Default|GetLiftMesh) (Math|Vector|Lerp(Vector) (Variables|Default|GetStart%20Point) (Variables|Default|GetEnd%20Point) _newtrack_0) false false)))))

(event OnComponentBeginOverlap(PlayerCheckCollider)
  (params (OverlappedComponent :type Primitive%20Component%20Object%20Reference) (OtherActor :type Actor%20Object%20Reference) (OtherComp :type Primitive%20Component%20Object%20Reference) (OtherBodyIndex :type Integer) (bFromSweep :type Boolean) (SweepResult :type Hit%20Result%20Structure%20%28by%20ref%29))
  (Utilities|Casting|CastToFirstPersonCharacter OtherActor)
  (Variables|Default|SetPlayerIsTrue true)
  (if (and (Variables|Default|GetCubeIsTrue) (Variables|Default|GetPlayerIsTrue))
    (bind _newtrack_0 (Timeline|Timeline_0 Play)
      (:Update
        (Transformation|SetRelativeLocation (Variables|Default|GetLiftMesh) (Math|Vector|Lerp(Vector) (Variables|Default|GetStart%20Point) (Variables|Default|GetEnd%20Point) _newtrack_0) false false)))))

(fn ConstructionScript)